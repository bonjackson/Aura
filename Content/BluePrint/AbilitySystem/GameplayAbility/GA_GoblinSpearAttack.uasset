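; Goblin spear melee gameplay ability that faces the combat target and plays a randomly picked attack montage.
; The montage's gameplay event triggers a small sphere query at its combat socket for live players.
; Non-friendly hits receive damage and a hit-effect gameplay cue, with one impact sound if anything was hit.
; The ability ends when the montage completes, blends out, is interrupted or cancelled, or cannot start.
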(event `self.K2_ActivateAbility`
  (bind _returnvalue (`self.GetAvatarActorFromActorInfo`))
  (bind _returnvalue_2 (`self.GetAvatarActorFromActorInfo`))
  (bind (_montage _montagetag) (break `TaggedMontage` (`self.Montage Struct`)))
  (set `self.HasHitTarget` false)
  (bind _returnvalue_3 (message `EnemyInterface.GetCombatTarget` _returnvalue))
  (bind _ascombat_interface (cast `CombatInterface` _returnvalue)
    (:`then`
      (`CombatInterface.UpdateFacingTarget` _ascombat_interface (`Actor.K2_GetActorLocation` _returnvalue_3))
      (bind _returnvalue_4 (message `CombatInterface.GetAttackMontages` (`self.GetAvatarActorFromActorInfo`)))
      (bind _returnvalue_5 (`KismetArrayLibrary.Array_Length` _returnvalue_4))
      (if (> _returnvalue_5 0)
        (bind _output_get (set `self.Montage Struct` (`|GetArrayItem` _returnvalue_4 (`KismetMathLibrary.RandomIntegerInRange` (- _returnvalue_5 1)))))
        (`AbilityTask_PlayMontageAndWait.CreatePlayMontageAndWaitProxy` "None" (`.Montage` (break `TaggedMontage` _output_get))
          (:`then`
            (`AbilityTask_WaitGameplayEvent.WaitGameplayEvent` _montagetag null
              (:`EventReceived`
                (bind _returnvalue_6 (message `CombatInterface.GetCombatSocketLocationByStruct` _returnvalue_2 _montagetag))
                (bind _outoverlappingactors (`AuraAbilitySystemLibrary.GetLivePlayersWithinRadius` _returnvalue_2 (`|MakeArray` _returnvalue_2) 45.0 _returnvalue_6))
                (for _array_element _outoverlappingactors
                  (if (`AuraAbilitySystemLibrary.IsNotFriend` _array_element (`self.GetAvatarActorFromActorInfo`))
                    (`self.CauseDamage` _array_element)
                    (set `self.HasHitTarget` true)
                    (`self.K2_ExecuteGameplayCueWithParams` (struct :`TagName` "GameplayCue.HitEffect") (`AbilitySystemBlueprintLibrary.MakeGameplayCueParameters` 0.0 0.0 (struct) (struct) (struct) (struct) (struct) (`Actor.K2_GetActorLocation` _array_element) (0.0 0.0 0.0) null null _array_element))))
                (if (`self.HasHitTarget`)
                  (`GameplayStatics.PlaySoundAtLocation` (`.ImpactSound` (break `TaggedMontage` (`self.Montage Struct`))) (`self.CombatLocation`) (struct) 1.0 1.0 0.0 null null null null)))))
          (:`OnCompleted`
            (`self.K2_EndAbility` :!label _label))
          (:`OnBlendOut`
            (goto _label))
          (:`OnInterrupted`
            (goto _label))
          (:`OnCancelled`
            (goto _label)))
        (else
          (`self.K2_EndAbility`))))
    (:`CastFailed`
      (`self.K2_EndAbility`))))